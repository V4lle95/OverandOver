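; Blueprint function library of shared helpers for a horror game.
; GetPlayer finds the Horror_Base child actor on the player character, and PlayerInput uses it to toggle input on that actor and the pawn, stopping movement when disabled.
; SetMesh applies a mesh with per-slot materials, optionally as dynamic instances with texture, color and emissive parameters.
; A search function returns the nearest actor of a given class to the player.
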(fn `GetPlayer`
  (returns (`As Master` :type "/Game/Horror/Blueprints/Core/Horror_Base Object Reference"))
  (bind _filteredarray (`KismetArrayLibrary.FilterArray` (`Actor.GetAllChildActors` (`GameplayStatics.GetPlayerCharacter` null) true) "/Game/Horror/Blueprints/Core/Horror_Base.Horror_Base_C"))
  (bind _ashorror_base (cast `/Game/Horror/Blueprints/Core/Horror_Base` (`|GetArrayItem` _filteredarray))
    (:`then`
      _)
    (:`CastFailed`
      (`KismetSystemLibrary.PrintString` null "Horror Base Not Attach To Camera" true true (struct :`R` 1.0 :`G` 0.013544 :`A` 1.0) 0.0)))
  (return _ashorror_base))

(fn `Nearest Actor to Player Of Class`
  (params (ActorClass :type "Actor Class Reference"))
  (returns (Success :type Boolean) (NearestActorOfClass :type "Actor Object Reference"))
  (locals (LocalFoundActor :type Boolean) (LocalNearestActor :type "Actor Object Reference") (LocalFloatComparison :type "Float (double-precision)"))
  (bind _outactors (`GameplayStatics.GetAllActorsOfClass` null ActorClass))
  (set `local.LocalFoundActor` (> (`KismetArrayLibrary.Array_Length` _outactors) 0))
  (bind _output (`|GetArrayItem` _outactors))
  (`/Engine/EditorBlueprintResources/StandardMacros.IsValid` _output
    (:`Is Valid`
      (set `local.LocalNearestActor` _output)
      (set `local.LocalFloatComparison` (`Actor.GetDistanceTo` _output (`GameplayStatics.GetPlayerCharacter` null)))
      (for _array_element _outactors
        (`/Engine/EditorBlueprintResources/StandardMacros.IsValid` _array_element
          (:`Is Valid`
            (bind _returnvalue (`Actor.GetDistanceTo` _array_element (`GameplayStatics.GetPlayerCharacter` null)))
            (if (< _returnvalue (`local.LocalFloatComparison`))
              (set `local.LocalFloatComparison` _returnvalue)
              (set `local.LocalNearestActor` _array_element)))))
      (return (`local.LocalFoundActor`) (`local.LocalNearestActor`)))))

(fn `PlayerInput`
  (params (Enable :type Boolean))
  (bind _returnvalue (`GameplayStatics.GetPlayerController` null))
  (bind _as_master (`self.GetPlayer` null))
  (if Enable
    (`Actor.EnableInput` _as_master _returnvalue)
    (`Actor.EnableInput` (`GameplayStatics.GetPlayerPawn` null) _returnvalue)
    (else
      (`Actor.DisableInput` _as_master _returnvalue)
      (`Actor.DisableInput` (`GameplayStatics.GetPlayerPawn` null) _returnvalue)
      (`MovementComponent.StopMovementImmediately` (`Pawn.GetMovementComponent` (`GameplayStatics.GetPlayerPawn` null))))))

(fn `SetMesh`
  (params (StaticMesh :type "StaticMeshComponent Object Reference") (MeshSettings :type "/Game/Horror/Blueprints/Structures/SetMesh/SetMesh Structure"))
  (bind (_mesh _materialsettings) (break `/Game/Horror/Blueprints/Structures/SetMesh/SetMesh` MeshSettings))
  (`StaticMeshComponent.SetStaticMesh` StaticMesh _mesh)
  (for _array_element _materialsettings
    (bind (_setmaterial _elementid _material _dynamicmaterial _dynamictexture _dynamiccolor _dynamicemissive) (break `/Game/Horror/Blueprints/Structures/SetMesh/SM_Material` _array_element))
    (if _setmaterial
      (if _dynamicmaterial
        (bind _returnvalue (`PrimitiveComponent.CreateDynamicMaterialInstance` StaticMesh _elementid _material "None"))
        (bind (_settexture _parametername _value) (break `/Game/Horror/Blueprints/Structures/SetMesh/SM_Texture` _dynamictexture))
        (if _settexture
          (`MaterialInstanceDynamic.SetTextureParameterValue` _returnvalue _parametername _value))
        (bind (_setcolor _parametername_2 _value_2) (break `/Game/Horror/Blueprints/Structures/SetMesh/SM_Color` _dynamiccolor))
        (if _setcolor
          (`MaterialInstanceDynamic.SetVectorParameterValue` _returnvalue _parametername_2 _value_2))
        (bind (_setemissive _parametername_3 _value_3) (break `/Game/Horror/Blueprints/Structures/SetMesh/SM_Emissive` _dynamicemissive))
        (if _setemissive
          (`MaterialInstanceDynamic.SetScalarParameterValue` _returnvalue _parametername_3 _value_3))
        (else
          (`PrimitiveComponent.SetMaterial` StaticMesh _elementid _material))))))