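; H_Events is a horror event actor that plays subtitle sequences from the HEvents data passed to HorrorEvent.
; HSubtitles spawns a separate H_Events actor for each sequence entry, so each entry runs its own delay in parallel.
; After its ModifyDurationOrSec delay, each spawned actor creates a W_Subtitle widget, adds it to the viewport and passes it the text.
; The file never destroys the spawned actors.
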(event `Horror Event`
  (params (`H events` :type "/Game/Horror/Blueprints/Structures/Events/H_events Structure"))
  (`self.H Subtitles` `H events`))

(event `H Subtitles`
  (params (`H Events` :type "/Game/Horror/Blueprints/Structures/Events/H_events Structure (by ref)"))
  (bind _addsequence (break `/Game/Horror/Blueprints/Structures/Events/Subtitles` (`.Subtitles_7_837A30294B181F49B27973B2495193F0` (break `/Game/Horror/Blueprints/Structures/Events/H_events` `H Events`))))
  (if (`KismetArrayLibrary.Array_IsValidIndex` _addsequence)
    (for _array_element _addsequence
      (bind _returnvalue (`|SpawnActorFromClass` "H_Events_C" (`KismetMathLibrary.MakeTransform` (0.0 0.0 0.0)) "DontSpawnIfColliding" "OverrideRootScale" null null))
      (`self.H Subtitle` _returnvalue _array_element))))

(event `H Subtitle`
  (params (Subtitle :type "/Game/Horror/Blueprints/Structures/Events/SubtitleSeq Structure"))
  (bind (_addsubtitle _modifyduration_or_sec) (break `/Game/Horror/Blueprints/Structures/Events/SubtitleSeq` Subtitle))
  (`KismetSystemLibrary.Delay` _modifyduration_or_sec)
  (bind _returnvalue (`|CreateWidget` "/Game/Horror/Widgets/W_Subtitle.W_Subtitle_C"))
  (`UserWidget.AddToViewport` _returnvalue 0)
  (`/Game/Horror/Widgets/W_Subtitle.SubtitleText` _returnvalue _addsubtitle 0))

(fn `UserConstructionScript`)