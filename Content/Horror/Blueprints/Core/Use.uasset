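; Base usable-object Blueprint for the horror game, with empty Use, Open/on and Close/Off events and a toggle for player input.
; HEventsCheck increments a counter on each HEvents entry and queues those reaching their AfterNTimes threshold, with separate handling for one-shot and repeating entries.
; It then spawns an H_Events actor per queued entry to run its horror event and clears the queue.
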(event `/Game/Horror/Blueprints/Core/Horror_BPI.Use`)

(event `/Game/Horror/Blueprints/Core/Horror_BPI.Open/on`)

(event `/Game/Horror/Blueprints/Core/Horror_BPI.Close/Off`)

(fn `ControllerInput`
  (params (Enable :type Boolean))
  (bind _returnvalue (`GameplayStatics.GetPlayerController` 0))
  (if Enable
    (`self.EnableInput` _returnvalue)
    (`self.EnableInput` (`GameplayStatics.GetPlayerCharacter` 0) _returnvalue)
    (else
      (`self.DisableInput` _returnvalue))))

(fn `H EventsCheck`
  (bind _h_events (`self.H Events`))
  (for (_array_element _array_index) _h_events
    (bind _structout (setmembers `/Game/Horror/Blueprints/Structures/Events/H_eventsMaster` :`StructRef` _array_element :`Counter` (+ (`.Counter_12_C1891E194B78BBC93548668BEF171A23` (break `/Game/Horror/Blueprints/Structures/Events/H_eventsMaster` _array_element)) 1)))
    (`KismetArrayLibrary.Array_Set` _h_events _array_index _structout)
    (bind (_afterntimes _counter _doonve) (break `/Game/Horror/Blueprints/Structures/Events/H_eventsMaster` _array_element))
    (if (== _afterntimes _counter)
      (`KismetArrayLibrary.Array_Add` (`self.IndexCache`) _array_index)
      (if _doonve
        (bind _structout_2 (setmembers `/Game/Horror/Blueprints/Structures/Events/H_eventsMaster` :`StructRef` _array_element))
        (`KismetArrayLibrary.Array_Set` _h_events _array_index _structout_2)
        (else
          (bind _structout_3 (setmembers `/Game/Horror/Blueprints/Structures/Events/H_eventsMaster` :`StructRef` _array_element :`Counter` 0))
          (`KismetArrayLibrary.Array_Set` _h_events _array_index _structout_3)))))
  (for _array_element_2 (`self.IndexCache`)
    (bind _returnvalue (`|SpawnActorFromClass` "/Game/Horror/Blueprints/Core/H_Events.H_Events_C" (`KismetMathLibrary.MakeTransform` (0.0 0.0 0.0)) "DontSpawnIfColliding" "OverrideRootScale" null null))
    (`/Game/Horror/Blueprints/Core/H_Events.Horror Event` _returnvalue (`.HEvents_17_837A30294B181F49B27973B2495193F0` (break `/Game/Horror/Blueprints/Structures/Events/H_eventsMaster` (`|GetArrayItem` (`self.H Events`) _array_element_2)))))
  (`KismetArrayLibrary.Array_Clear` (`self.IndexCache`)))

(fn `UserConstructionScript`)