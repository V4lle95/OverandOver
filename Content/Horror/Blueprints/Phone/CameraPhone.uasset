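; CameraPhone is a phone Blueprint for a horror game with a scene-capture camera and a toggleable flashlight.
; The F key toggles two spotlights and the flashlight component together and plays a switch sound attached to the phone.
; Holding right mouse runs a timeline that narrows the capture FOV toward half of normal for zoom, reversing on release.
; The construction script tints the flashlight's dynamic material to match the spotlight's color.
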(event `self.ReceiveBeginPlay`
  (`self.ControllerInput` true))

(event `Key|F`
  (params (Key :type "Key Structure"))
  (bind _spotlight (`self.SpotLight`))
  (:`Pressed`
    (`SceneComponent.SetVisibility` _spotlight (not (`SceneComponent.bVisible` _spotlight)) false)
    (`SceneComponent.SetVisibility` (`self.Flashlight`) (not (`SceneComponent.bVisible` _spotlight)) false)
    (`SceneComponent.SetVisibility` (`self.SpotLight1`) (not (`SceneComponent.bVisible` _spotlight)) false)
    (`/Game/Horror/Blueprints/Core/HR_Macros.3DSound` null true "/Game/Horror/Blueprints/Phone/Sound/Flashlight_Switch.Flashlight_Switch" (`self.Phone`))))

(event `Key|RightMouseButton`
  (params (Key :type "Key Structure"))
  (bind _normal_fov (`self.Normal FOV`))
  (:`Pressed`
    (bind (_direction _alpha) (`Timeline|FOV TL`)
      (:`Update`
        (set `SceneCaptureComponent2D.FOVAngle` (`KismetMathLibrary.Lerp` _normal_fov (/ _normal_fov 2.0) _alpha) (`self.SceneCaptureComponent2D`)))))
  (:`Released`
    (`TimelineComponent.Reverse` (`self.FOV TL`))))

(fn `UserConstructionScript`
  (bind (_r _g _b) (break `LinearColor` (`KismetMathLibrary.Conv_ColorToLinearColor` (`LightComponentBase.LightColor` (`self.SpotLight`)))))
  (bind _returnvalue (`PrimitiveComponent.CreateDynamicMaterialInstance` (`self.Flashlight`) 0 null "None"))
  (`MaterialInstanceDynamic.SetVectorParameterValue` _returnvalue "Color" (make `LinearColor` _r _g _b 0.8)))