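; CheckShards is a manager actor that tracks how many shards remain in the level.
; On BeginPlay it attaches every actor of a class to itself, takes the attached-actor count as the shard total and copies it to the player.
; RemoveShard decrements that total and updates the player's copy.
; A fast looping timer polls the count through CheckMax and destroys the manager when none remain.
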(event `self.ReceiveBeginPlay`
  (bind _outactors (`GameplayStatics.GetAllActorsOfClass` null))
  (`self.K2_AttachToActor` _outactors self "None" "KeepWorld" "KeepWorld" "KeepWorld" true)
  (set `self.Shards In Level` (`KismetArrayLibrary.Array_Length` (`self.GetAttachedActors` true)))
  (bind _as_master (`/Game/Horror/Blueprints/Core/Horror_funtions.GetPlayer`))
  (set `/Game/Horror/Blueprints/Core/Horror_Base.ShardsInLevel` (`self.Shards In Level`) _as_master)
  (`KismetSystemLibrary.K2_SetTimer` null "Check Max" 0.1 true))

(event `Check Max`
  (if (== (`self.Shards In Level`) 0)
    (`self.K2_DestroyActor`)))

(fn `Remove Shard`
  (set `self.Shards In Level` (- (`self.Shards In Level`) 1))
  (bind _as_master (`/Game/Horror/Blueprints/Core/Horror_funtions.GetPlayer`))
  (set `/Game/Horror/Blueprints/Core/Horror_Base.ShardsInLevel` (`self.Shards In Level`) _as_master))

(fn `UserConstructionScript`)