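; BP_WorldCapture defines a minimap capture area with an orthographic scene capture and a trigger box.
; The construction script places two corner spheres and the trigger, then sets OrthoWidth to the corners' larger X or Y separation.
; Player overlap writes that width to the Minimap_data parameter collection as Dimensions.
; Render target creation and brief capture logic is unconnected, and SizeCapture only prints the width.
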(event `self.ReceiveBeginPlay`)

(event `Size Capture`
  (`KismetSystemLibrary.PrintString` (`KismetStringLibrary.Conv_DoubleToString` (`SceneCaptureComponent2D.OrthoWidth` (`self.SceneCapture`))) true true (struct :`R` 1.0 :`G` 1.0 :`B` 1.0 :`A` 1.0) -1.0))

(event `self.Trigger.OnComponentBeginOverlap`
  (params (OverlappedComponent :type "PrimitiveComponent Object Reference") (OtherActor :type "Actor Object Reference") (OtherComp :type "PrimitiveComponent Object Reference") (OtherBodyIndex :type Integer) (bFromSweep :type Boolean) (SweepResult :type "HitResult Structure (by ref)"))
  (bind _returnvalue (== OtherActor (`GameplayStatics.GetPlayerPawn` 0)))
  (if _returnvalue
    (`KismetMaterialLibrary.SetScalarParameterValue` "/Game/Horror/Materials/Minimap_data.Minimap_data" "Dimensions" (`SceneCaptureComponent2D.OrthoWidth` (`self.SceneCapture`)))
    (`KismetSystemLibrary.PrintString` (`KismetStringLibrary.Conv_BoolToString` _returnvalue))))

(fn `UserConstructionScript`
  (bind _trigger (`self.Trigger`))
  (bind (_returnvalue_x _returnvalue_y) (`KismetMathLibrary.BreakVector` (`SceneComponent.K2_GetComponentLocation` (`self.Lower Right Sphere`))))
  (bind (_returnvalue_x_2 _returnvalue_y_2) (`KismetMathLibrary.BreakVector` (`SceneComponent.K2_GetComponentLocation` (`self.Upper Left Sphere`))))
  (`|ExecutionSequence`
    (:`then_0`
      (`SceneComponent.K2_SetRelativeLocation` (`self.Upper Left Sphere`) (`self.Upper Left Sphere Loc`) false false)
      (`SceneComponent.K2_SetRelativeLocation` (`self.Lower Right Sphere`) (`self.Lower Right Sphere Loc`) false false)
      (`SceneComponent.K2_SetRelativeLocation` _trigger (`self.Trigger Loc`) false false)
      (`BoxComponent.SetBoxExtent` _trigger (`self.Trigger Size`) true))
    (:`then_1`
      (set `SceneCaptureComponent2D.OrthoWidth` (`KismetMathLibrary.FMax` (`KismetMathLibrary.Abs` (- _returnvalue_x _returnvalue_x_2)) (`KismetMathLibrary.Abs` (- _returnvalue_y _returnvalue_y_2))) (`self.SceneCapture`)))))